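; Interactable safe that opens through a dial-lock puzzle and holds a key for pickup.
; Sphere overlaps toggle prompt widgets and outline overlay materials on the safe or key, depending on open and pickup state.
; EInteraction opens the dial-lock widget with UI-only input, or hides and flags the key once open.
; Widget callbacks restore game input on close, or play the opening animation (frozen at BeginPlay) and a sound on a correct code.
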(event OnComponentBeginOverlap(Sphere)
  (params (OverlappedComponent :type Primitive%20Component%20Object%20Reference) (OtherActor :type Actor%20Object%20Reference) (OtherComp :type Primitive%20Component%20Object%20Reference) (OtherBodyIndex :type Integer) (bFromSweep :type Boolean) (SweepResult :type Hit%20Result%20Structure%20%28by%20ref%29))
  ;[1 1 1] E
  (if (Variables|Default|GetIsSafeOpen)
    (if (not (Variables|Default|GetIsKeyPickedUp))
      (Rendering|SetVisibility (Variables|Default|GetWidgetE2) true false)
      (Rendering|Material|SetOverlayMaterial (Variables|Default|GetKey) "/Game/Materials/Outline.Outline" :!class /Script/Engine.MeshComponent))
    (else
      (Rendering|SetVisibility (Variables|Default|GetWidgetE1) true false)
      (Rendering|Material|SetOverlayMaterial (Variables|Default|GetSafeMesh) "/Game/Materials/Outline.Outline" :!class /Script/Engine.MeshComponent))))

(event OnComponentEndOverlap(Sphere)
  (params (OverlappedComponent :type Primitive%20Component%20Object%20Reference) (OtherActor :type Actor%20Object%20Reference) (OtherComp :type Primitive%20Component%20Object%20Reference) (OtherBodyIndex :type Integer))
  ;[1 1 1] E
  (if (Variables|Default|GetIsSafeOpen)
    (if (Variables|Default|GetIsKeyPickedUp)
      (Rendering|SetVisibility (Variables|Default|GetWidgetE2) false false)
      (Rendering|Material|SetOverlayMaterial (Variables|Default|GetKey) (Variables|Default|GetOriginalMaterial) :!class /Script/Engine.MeshComponent))
    (else
      (Rendering|SetVisibility (Variables|Default|GetWidgetE1) false false)
      (Rendering|Material|SetOverlayMaterial (Variables|Default|GetSafeMesh) (Variables|Default|GetOriginalMaterial) :!class /Script/Engine.MeshComponent))))

(event Custom|UnlockSafe
  (Rendering|Material|SetOverlayMaterial (Variables|Default|GetKey) "/Game/Materials/Outline.Outline" :!class /Script/Engine.MeshComponent)
  (Components|Animation|PlayAnimation (Variables|Default|GetSafeMesh) "/Game/Models/Safe/scene_Anim.scene_Anim" false)
  (Variables|Default|SetIsSafeOpen true)
  (Rendering|SetVisibility (Variables|Default|GetWidgetE1) false false)
  (Audio|PlaySound2D "/Game/Audio/Dialogue/Notes.Notes" 1.0 1.0 0.0 0 0)
  (Development|PrintString "UNLOCKED"))

(event Custom|Close
  (bind _returnvalue (Game|GetPlayerController 0))
  (Variables|Default|SetIsUIShowing false)
  (Widget|RemovefromParent (stale EventEInteraction _returnvalue_2))
  (Input|SetInputModeGameOnly _returnvalue false)
  (Variables|/Script/Engine.PlayerController|SetbShowMouseCursor _returnvalue false)
  (Development|PrintString "Closed"))

(event EventBeginPlay
  (bind _safemesh (Variables|Default|GetSafeMesh))
  (Components|Animation|PlayAnimation _safemesh "/Game/Models/Safe/scene_Anim.scene_Anim" false)
  (Development|PrintString "Anim Paused on start")
  (Components|Timeline|SetPlayRate _safemesh 0.0))

(event EventEInteraction
  (bind _returnvalue (Game|GetPlayerController 0))
  (if (Variables|Default|GetIsSafeOpen)
    (if (not (Variables|Default|GetIsKeyPickedUp))
      (Variables|Default|SetIsKeyPickedUp true)
      (Rendering|SetVisibility (Variables|Default|GetKey) false false)
      (Rendering|SetVisibility (Variables|Default|GetWidgetE2) false false)
      (Development|PrintString "Key Picked Up!"))
    (elif (not (Variables|Default|GetIsUIShowing))
      (Variables|Default|SetIsUIShowing true)
      (Rendering|Material|SetOverlayMaterial (Variables|Default|GetSafeMesh) (Variables|Default|GetOriginalMaterial) :!class /Script/Engine.MeshComponent)
      (bind _returnvalue_2 (UserInterface|CreateWidget "/Game/UI/DialLockWidget.DialLockWidget_C"))
      (EventDispatchers|BindEventtoCloseButtonEvent _returnvalue_2 (delegate Custom|Close))
      (UserInterface|Viewport|AddtoViewport _returnvalue_2 0)
      (Input|SetInputModeUIOnly _returnvalue 0 "DoNotLock" false)
      (Variables|/Script/Engine.PlayerController|SetbShowMouseCursor _returnvalue true)
      (EventDispatchers|BindEventtoOnCodeCorrect _returnvalue_2 (delegate Custom|UnlockSafe)))))

(fn ConstructionScript)