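; Window door Blueprint that swings open by driving a scene component's yaw with the OpenWindow timeline.
; Overlapping the sphere plays the timeline directly, with no key check.
; Interaction_1 also plays it, once, if SafeBP reports the key picked up, setting IsOpen and hiding the WidgetE1 widget.
; Leaving the sphere hides that widget; the logic that would show it is unconnected.
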(event OnComponentBeginOverlap(Sphere)
  (params (OverlappedComponent :type Primitive%20Component%20Object%20Reference) (OtherActor :type Actor%20Object%20Reference) (OtherComp :type Primitive%20Component%20Object%20Reference) (OtherBodyIndex :type Integer) (bFromSweep :type Boolean) (SweepResult :type Hit%20Result%20Structure%20%28by%20ref%29))
  (bind _rotationvalue (Timeline|OpenWindow Play)
    (:Update
      (Transformation|SetRelativeRotation (Variables|Default|GetSceneComponent) (Math|Rotator|MakeRotator 0.0 0.0 _rotationvalue) false false))
    (:Finished
      (Development|PrintString "Lock Opened"))))

(event OnComponentEndOverlap(Sphere)
  (params (OverlappedComponent :type Primitive%20Component%20Object%20Reference) (OtherActor :type Actor%20Object%20Reference) (OtherComp :type Primitive%20Component%20Object%20Reference) (OtherBodyIndex :type Integer))
  (if (Variables|/Game/Blueprints/SafeBP.SafeBP_C|GetIsKeyPickedUp (Variables|Default|GetSafeBP))
    _
    (else
      _))
  (Rendering|SetVisibility (Variables|Default|GetWidgetE1) false false))

(event Custom|Interaction_1
  (if (not (Variables|Default|GetIsOpen))
    (if (Variables|/Game/Blueprints/SafeBP.SafeBP_C|GetIsKeyPickedUp (Variables|Default|GetSafeBP))
      (Variables|Default|SetIsOpen true)
      (Rendering|SetVisibility (Variables|Default|GetWidgetE1) false false)
      (bind _rotationvalue (Timeline|OpenWindow Play)
        (:Update
          (Transformation|SetRelativeRotation (Variables|Default|GetSceneComponent) (Math|Rotator|MakeRotator 0.0 0.0 _rotationvalue) false false))
        (:Finished
          (Development|PrintString "Lock Opened"))))))

(fn ConstructionScript)