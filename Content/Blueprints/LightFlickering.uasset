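; Light flicker Blueprint that makes its PointLight flash at random intensities.
; BeginPlay starts a looping timer whose period is randomized only once, calling FlickerLight each time.
; FlickerLight sets a random intensity, waits a random delay, then switches the light to zero.
; Delay durations use variables named as intensity ranges, and the final delay leads to nothing, so the timer alone drives repetition.
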(event Custom|FlickerLight
  (Rendering|Components|Light|SetIntensity (Variables|Default|GetPointLight) (Math|Random|RandomFloatinRange (Variables|Default|GetFlickerIntensityMin%20) (Variables|Default|GetFlickerIntensityMax%20)))
  (Utilities|FlowControl|Delay (Math|Random|RandomFloatinRange (Variables|Default|GetFlickerIntensityMin2) (Variables|Default|GetFlickerIntensityMax2)))
  (Rendering|Components|Light|SetIntensity (Variables|Default|GetPointLight) 0.0)
  (Utilities|FlowControl|Delay (Math|Random|RandomFloatinRange (Variables|Default|GetFlickerIntensityMin3) (Variables|Default|GetFlickerIntensityMax3))))

(event EventBeginPlay
  (Utilities|Time|SetTimerbyEvent (delegate Custom|FlickerLight) (Math|Random|RandomFloatinRange 0.1 (Variables|Default|GetFlickerInteraval)) true))

(fn ConstructionScript)