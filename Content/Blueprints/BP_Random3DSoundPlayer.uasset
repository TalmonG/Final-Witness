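; Ambient sound actor that plays random 3D sounds near the player at random intervals.
; From BeginPlay, a self-calling event waits roughly 20 to 60 seconds, picks a sound from an array, then moves its root to a random world-axis offset from the player.
; It then plays the audio component and prints a debug message.
; The separate PlayRandomSound function is uncalled, with its sound selection and playback nodes disconnected.
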(event Custom|PlayRandomSoundLoop
  (bind _returnvalue (Game|GetPlayerCharacter 0))
  (bind _array (Variables|Default|GetArray))
  (bind _returnvalue_2 (Transformation|GetActorLocation _returnvalue))
  (bind (_x _y _z) (Math|Vector|BreakVector _returnvalue_2))
  (Utilities|FlowControl|Delay (Math|Random|RandomFloatinRange 6e+01 2e+01))
  (Audio|Components|Audio|SetSound (Variables|Default|GetAudio) (Utilities|Array|Get(acopy) _array (Math|Random|RandomIntegerinRange 0 (- (Utilities|Array|Length _array) 1))))
  (Transformation|SetWorldLocation (Variables|Default|GetDefaultSceneRoot) (Math|Vector|MakeVector (- _x (Math|Random|RandomFloatinRange 0.0 -5e+01)) (- _y (Math|Random|RandomFloatinRange -1e+02 1e+02)) _z) false false)
  (Audio|Components|Audio|Play (Variables|Default|GetAudio) 0.0)
  (Development|PrintString "Sound Played")
  (CallFunction|PlayRandomSoundLoop))

(event EventBeginPlay
  (CallFunction|PlayRandomSoundLoop))

(fn ConstructionScript)

(fn PlayRandomSound
  (bind _returnvalue (Game|GetPlayerCharacter 0))
  (bind _returnvalue_2 (Transformation|GetActorLocation _returnvalue))
  (bind (_x _y _z) (Math|Vector|BreakVector _returnvalue_2))
  (Transformation|SetWorldLocation (Variables|Default|GetDefaultSceneRoot) (Math|Vector|MakeVector _x (- _y -1e+02) _z) false false))