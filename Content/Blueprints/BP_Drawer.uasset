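; BP_Drawer is an interactable drawer that opens to reveal a note the player can view on screen.
; Sphere overlap toggles an interaction prompt and outline overlay on the drawer, or on the note once opened.
; The first EInteraction plays a sound and slides the drawer along X via a timeline.
; Later interactions toggle between showing an animated note widget in the viewport and removing it.
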(event OnComponentBeginOverlap(Sphere1)
  (params (OverlappedComponent :type Primitive%20Component%20Object%20Reference) (OtherActor :type Actor%20Object%20Reference) (OtherComp :type Primitive%20Component%20Object%20Reference) (OtherBodyIndex :type Integer) (bFromSweep :type Boolean) (SweepResult :type Hit%20Result%20Structure%20%28by%20ref%29))
  ;[1 1 1] 1st E
  (if (Variables|Default|GetIsOpenedMain)
    (Rendering|SetVisibility (Variables|Default|GetWidgetE2) true false)
    (Rendering|Material|SetOverlayMaterial (Variables|Default|GetNoteSlideUpAnim) "/Game/Materials/Outline.Outline" :!class /Script/Engine.MeshComponent)
    (else
      (Rendering|SetVisibility (Variables|Default|GetWidgetE1) true false)
      (Rendering|Material|SetOverlayMaterial (Variables|Default|GetMainDraw) "/Game/Materials/Outline.Outline" :!class /Script/Engine.MeshComponent))))

(event OnComponentEndOverlap(Sphere1)
  (params (OverlappedComponent :type Primitive%20Component%20Object%20Reference) (OtherActor :type Actor%20Object%20Reference) (OtherComp :type Primitive%20Component%20Object%20Reference) (OtherBodyIndex :type Integer))
  ;[1 1 1] 1st E
  (if (Variables|Default|GetIsOpenedMain)
    (Rendering|SetVisibility (Variables|Default|GetWidgetE2) false false)
    (Rendering|Material|SetOverlayMaterial (Variables|Default|GetNoteSlideUpAnim) (Variables|Default|GetOriginalMaterial) :!class /Script/Engine.MeshComponent)
    (else
      (Rendering|SetVisibility (Variables|Default|GetWidgetE1) false false)
      (Rendering|Material|SetOverlayMaterial (Variables|Default|GetMainDraw) (Variables|Default|GetOriginalMaterial) :!class /Script/Engine.MeshComponent))))

(event Custom|Interaction_1)

(event EventEInteraction
  (if (Variables|Default|GetIsOpenedMain)
    (if (Variables|Default|GetIsNotePickedUp)
      (Variables|Default|SetIsNotePickedUp false)
      (Rendering|Material|SetOverlayMaterial (Variables|Default|GetNoteSlideUpAnim) "/Game/Materials/Outline.Outline" :!class /Script/Engine.MeshComponent)
      (Widget|RemovefromParent (Variables|Default|GetNoteAnimWidget))
      (Development|PrintString "Put Down")
      (else
        (Variables|Default|SetIsNotePickedUp true)
        (Rendering|Material|SetOverlayMaterial (Variables|Default|GetMainDraw) (Variables|Default|GetOriginalMaterial) :!class /Script/Engine.MeshComponent)
        (bind _returnvalue (UserInterface|CreateWidget "/Game/UI/NoteAnim.NoteAnim_C"))
        (bind _output_get (Variables|Default|SetNoteAnimWidget _returnvalue))
        (UserInterface|Viewport|AddtoViewport _output_get 0)
        (UserInterface|Animation|PlayAnimation (Variables|Default|GetNoteAnimWidget) 0 0.0 1 "Forward" 1.0 false)))
    (else
      ;[1 1 1] DrawOpen
      (Variables|Default|SetIsOpenedMain true)
      (Rendering|Material|SetOverlayMaterial (Variables|Default|GetMainDraw) (Variables|Default|GetOriginalMaterial) :!class /Script/Engine.MeshComponent)
      (Rendering|SetVisibility (Variables|Default|GetWidgetE1) false false)
      (Audio|PlaySound2D "/Game/Audio/Dialogue/Notes.Notes" 1.0 1.0 0.0 0 0)
      (bind _drawerposition (Timeline|OpenDraw Play)
        (:Update
          (Transformation|SetRelativeLocation (Variables|Default|GetMainDraw) (Math|Vector|MakeVector _drawerposition 0.0 0.0) false false)
          (Rendering|SetVisibility (Variables|Default|GetWidgetE2) true false))))))

(fn ConstructionScript)