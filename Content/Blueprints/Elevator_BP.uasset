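; Elevator Blueprint that the player triggers with E, with input enabled on overlapping its Box and disabled on leaving.
; Timelines close the Gates, move SharedRoot along the room track, then reopen the gates, with audio components added at start and arrival.
; Room movement starts from the gate timeline's Update, so it overlaps the closing.
; Only FlipFlop's A output is wired, so alternate presses do nothing and no return trip exists.
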(event OnComponentBeginOverlap(Box)
  (params (OverlappedComponent :type Primitive%20Component%20Object%20Reference) (OtherActor :type Actor%20Object%20Reference) (OtherComp :type Primitive%20Component%20Object%20Reference) (OtherBodyIndex :type Integer) (bFromSweep :type Boolean) (SweepResult :type Hit%20Result%20Structure%20%28by%20ref%29))
  (Input|EnableInput (Game|GetPlayerController 0)))

(event OnComponentEndOverlap(Box)
  (params (OverlappedComponent :type Primitive%20Component%20Object%20Reference) (OtherActor :type Actor%20Object%20Reference) (OtherComp :type Primitive%20Component%20Object%20Reference) (OtherBodyIndex :type Integer))
  (Input|DisableInput (Game|GetPlayerController 0)))

(event Input|KeyboardEvents|E
  (params (Key :type Key%20Structure :default "None"))
  (:Pressed
    (Utilities|FlowControl|FlipFlop
      (:A
        (AddComponent|AddAudioComponent false)
        (bind _gatesclose__1 (Timeline|ElevatorAnim Play)
          (:Update
            (Transformation|SetRelativeLocation (Variables|Default|GetGates) _gatesclose__1 false false)
            (bind _elevatorroom (Timeline|Timeline Play)
              (:Update
                (Transformation|SetRelativeLocation (Variables|Default|GetSharedRoot) _elevatorroom false false))
              (:Finished
                (AddComponent|AddAudioComponent false)
                (bind _gatesopen__1 (Timeline|Timeline_2 Play)
                  (:Update
                    (Transformation|SetRelativeLocation (Variables|Default|GetGates) _gatesopen__1 false false)))))))))))

(fn ConstructionScript)