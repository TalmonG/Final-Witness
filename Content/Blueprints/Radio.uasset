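; Interactable radio Blueprint that plays a random sound from its array at BeginPlay and toggles off or on with each interaction.
; A sphere overlap shows a widget and applies an outline overlay material to the frame, reverting both on exit.
; EInteraction shares BeginPlay's FlipFlop, alternately stopping the speaker or starting a new pick at a random whole-second offset.
; That offset's upper bound comes from a separately randomized array entry's duration.
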(event OnComponentBeginOverlap(Sphere)
  (params (OverlappedComponent :type Primitive%20Component%20Object%20Reference) (OtherActor :type Actor%20Object%20Reference) (OtherComp :type Primitive%20Component%20Object%20Reference) (OtherBodyIndex :type Integer) (bFromSweep :type Boolean) (SweepResult :type Hit%20Result%20Structure%20%28by%20ref%29))
  ;[1 1 1] Comment
  (Rendering|SetVisibility (Variables|Default|GetWidgetE) true false)
  (Rendering|Material|SetOverlayMaterial (Variables|Default|GetFrame) "/Game/Materials/Outline.Outline" :!class /Script/Engine.MeshComponent))

(event OnComponentEndOverlap(Sphere)
  (params (OverlappedComponent :type Primitive%20Component%20Object%20Reference) (OtherActor :type Actor%20Object%20Reference) (OtherComp :type Primitive%20Component%20Object%20Reference) (OtherBodyIndex :type Integer))
  ;[1 1 1] Comment
  (Rendering|SetVisibility (Variables|Default|GetWidgetE) false false)
  (Rendering|Material|SetOverlayMaterial (Variables|Default|GetFrame) (Variables|Default|GetOriginalMaterial) :!class /Script/Engine.MeshComponent))

(event EventEInteraction
  (bind _array (Variables|Default|GetArray))
  (bind _returnvalue (Utilities|Array|Length _array))
  (bind _returnvalue_2 (- _returnvalue 1))
  (bind _returnvalue_3 (Math|Random|RandomIntegerinRange 0 _returnvalue_2))
  (bind _output (Utilities|Array|Get(acopy) _array _returnvalue_3))
  (Utilities|FlowControl|FlipFlop
    (:A
      (Audio|Components|Audio|SetSound (Variables|Default|GetSpeaker) _output)
      (Audio|Components|Audio|Play (Variables|Default|GetSpeaker) (Math|Conversions|ToFloat(Integer) (Math|Random|RandomIntegerinRange 1 (Math|Float|Truncate (Variables|/Script/Engine.SoundBase|GetDuration _output))))))
    (:B
      (Audio|Components|Audio|Stop (Variables|Default|GetSpeaker)))))

(event EventBeginPlay
  (bind _array (Variables|Default|GetArray))
  (bind _returnvalue (Utilities|Array|Length _array))
  (bind _returnvalue_2 (- _returnvalue 1))
  (bind _returnvalue_3 (Math|Random|RandomIntegerinRange 0 _returnvalue_2))
  (bind _output (Utilities|Array|Get(acopy) _array _returnvalue_3))
  (Utilities|FlowControl|FlipFlop
    (:A
      (Audio|Components|Audio|SetSound (Variables|Default|GetSpeaker) _output)
      (Audio|Components|Audio|Play (Variables|Default|GetSpeaker) (Math|Conversions|ToFloat(Integer) (Math|Random|RandomIntegerinRange 1 (Math|Float|Truncate (Variables|/Script/Engine.SoundBase|GetDuration _output))))))
    (:B
      (Audio|Components|Audio|Stop (Variables|Default|GetSpeaker)))))

(fn ConstructionScript)