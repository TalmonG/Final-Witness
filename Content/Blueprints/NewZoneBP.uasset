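; NewZoneBP is a one-shot trigger zone that announces Chapter 1 with an on-screen title and dramatic audio.
; The first Box overlap by any actor sets IsCollided, so later overlaps are ignored.
; After a zero-length delay, it creates a MessageWidget, fills in the hardcoded chapter title and quote, adds it to the viewport and plays two 2D sounds, Thunder and DoomDoom.
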(event OnComponentBeginOverlap(Box)
  (params (OverlappedComponent :type Primitive%20Component%20Object%20Reference) (OtherActor :type Actor%20Object%20Reference) (OtherComp :type Primitive%20Component%20Object%20Reference) (OtherBodyIndex :type Integer) (bFromSweep :type Boolean) (SweepResult :type Hit%20Result%20Structure%20%28by%20ref%29))
  (if (not (Variables|Default|GetIsCollided))
    (Variables|Default|SetIsCollided true)
    (Utilities|FlowControl|Delay 0.0)
    (bind _returnvalue (UserInterface|CreateWidget "/Game/UI/MessageWidget/MessageWidget.MessageWidget_C"))
    (Variables|Default|SetMessageWidgetRef _returnvalue)
    (Default|SetMessage (Variables|Default|GetMessageWidgetRef) "Chapter 1" "\"It's like she's in the walls\"")
    (UserInterface|Viewport|AddtoViewport (Variables|Default|GetMessageWidgetRef) 0)
    (Audio|PlaySound2D "/Game/Audio/Thunder.Thunder" 1.0 1.0 0.0 0 0)
    (Audio|PlaySound2D "/Game/Audio/SoundEffects/DoomDoom.DoomDoom" 1.0 1.0 0.0 0 0)))

(event OnComponentEndOverlap(Box)
  (params (OverlappedComponent :type Primitive%20Component%20Object%20Reference) (OtherActor :type Actor%20Object%20Reference) (OtherComp :type Primitive%20Component%20Object%20Reference) (OtherBodyIndex :type Integer)))

(fn ConstructionScript)